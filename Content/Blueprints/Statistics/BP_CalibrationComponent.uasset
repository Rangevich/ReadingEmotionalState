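; Actor component that turns a user's recorded statistics into averaged calibration values stored on the Game Instance.
; Each save function averages one data map from the owner's BP_UserStatisticsComponent and passes the result to the Game Instance through a message call.
; SaveCalibration runs the pawn speed, input count and fast turn saves.
; SaveTurnSpeed follows the same pattern but is not called by SaveCalibration.
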(event `SaveCalibration`
  (`self.SavePawnSpeed`)
  (`self.SaveInputCount`)
  (`self.SaveFastTurn`))

(fn `SaveFastTurn`
  (locals (FastTurn :type "Float (double-precision)"))
  (bind _values (`BlueprintMapLibrary.Map_Values` (`/Game/Blueprints/Statistics/BP_UserStatisticsComponent.FastTurnData` (`Actor.GetComponentByClass` (`self.GetOwner`) "/Game/Blueprints/Statistics/BP_UserStatisticsComponent.BP_UserStatisticsComponent_C"))))
  (for _array_element _values
    (set `local.FastTurn` (+ _array_element (`local.FastTurn`))))
  (bind _output_get (set `local.FastTurn` (/ (`local.FastTurn`) (`KismetArrayLibrary.Array_Length` _values))))
  (message `/Game/Blueprints/BPI_UserData.SetAverageFastTurnCount` (`GameplayStatics.GetGameInstance`) _output_get))

(fn `SaveInputCount`
  (locals (InputCount :type "Float (double-precision)"))
  (bind _values (`BlueprintMapLibrary.Map_Values` (`/Game/Blueprints/Statistics/BP_UserStatisticsComponent.InputData` (`Actor.GetComponentByClass` (`self.GetOwner`) "/Game/Blueprints/Statistics/BP_UserStatisticsComponent.BP_UserStatisticsComponent_C"))))
  (for _array_element _values
    (set `local.InputCount` (+ _array_element (`local.InputCount`))))
  (bind _output_get (set `local.InputCount` (/ (`local.InputCount`) (`KismetArrayLibrary.Array_Length` _values))))
  (message `/Game/Blueprints/BPI_UserData.SetAverageInputCount` (`GameplayStatics.GetGameInstance`) _output_get))

(fn `SavePawnSpeed`
  (locals (pawnSpeed :type "Float (double-precision)"))
  (bind _values (`BlueprintMapLibrary.Map_Values` (`/Game/Blueprints/Statistics/BP_UserStatisticsComponent.PawnSpeedData` (`Actor.GetComponentByClass` (`self.GetOwner`) "/Game/Blueprints/Statistics/BP_UserStatisticsComponent.BP_UserStatisticsComponent_C"))))
  (for _array_element _values
    (set `local.pawnSpeed` (+ _array_element (`local.pawnSpeed`))))
  (bind _output_get (set `local.pawnSpeed` (/ (`local.pawnSpeed`) (`KismetArrayLibrary.Array_Length` _values))))
  (message `/Game/Blueprints/BPI_UserData.SetAveragePawnSpeed` (`GameplayStatics.GetGameInstance`) _output_get))

(fn `SaveTurnSpeed`
  (locals (turnSpeed :type "Float (double-precision)"))
  (bind _values (`BlueprintMapLibrary.Map_Values` (`/Game/Blueprints/Statistics/BP_UserStatisticsComponent.TurnSpeedData` (`Actor.GetComponentByClass` (`self.GetOwner`) "/Game/Blueprints/Statistics/BP_UserStatisticsComponent.BP_UserStatisticsComponent_C"))))
  (for _array_element _values
    (set `local.turnSpeed` (+ _array_element (`local.turnSpeed`))))
  (bind _output_get (set `local.turnSpeed` (/ (`local.turnSpeed`) (`KismetArrayLibrary.Array_Length` _values))))
  (message `/Game/Blueprints/BPI_UserData.SetAverageTurnSpeed` (`GameplayStatics.GetGameInstance`) _output_get))