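; Player controller component that records player behavior per map location and turns it into a heatmap snapshot.
; After a short delay, Tick fills maps keyed by grid-snapped pawn XY with peak turn speed, pawn speed and key-press input, plus fast-turn counts.
; SaveDataPhoto compares these against GameInstance averages, blends clamped excesses into heat values, then spawns BP_ProbeActor per cell and BP_SnapshotCamera at the Snapshot-tagged actor.
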(event `self.ReceiveBeginPlay`
  (bind _asplayer_controller (cast `PlayerController` (`self.GetOwner`)))
  (set `self.PlayerControllerOwner` _asplayer_controller)
  (`KismetSystemLibrary.K2_SetTimerDelegate` (delegate `StartTick`) 0.5))

(event `StartTick`
  (`self.SetComponentTickEnabled` true))

(event `self.ReceiveTick`
  (params (DeltaSeconds :type "Float (single-precision)"))
  (`self.CalculateTurnSpeed`)
  (`self.CheckFastTurn`)
  (`self.AddInputData`)
  (`self.AddPawnSpeedData`))

(event `Key|W` :consume false :overrideparent false
  (params (Key :type "Key Structure"))
  (:`Pressed`
    (`/Engine/EditorBlueprintResources/StandardMacros.IncrementInt` (`self.TimedInputCounter`))))

(event `Key|A` :consume false :overrideparent false
  (params (Key :type "Key Structure"))
  (:`Pressed`
    (`/Engine/EditorBlueprintResources/StandardMacros.IncrementInt` (`self.TimedInputCounter`))))

(event `Key|S` :consume false :overrideparent false
  (params (Key :type "Key Structure"))
  (:`Pressed`
    (`/Engine/EditorBlueprintResources/StandardMacros.IncrementInt` (`self.TimedInputCounter`))))

(event `Key|D` :consume false :overrideparent false
  (params (Key :type "Key Structure"))
  (:`Pressed`
    (`/Engine/EditorBlueprintResources/StandardMacros.IncrementInt` (`self.TimedInputCounter`))))

(event `Key|F` :consume false :overrideparent false
  (params (Key :type "Key Structure"))
  (:`Pressed`
    (`/Engine/EditorBlueprintResources/StandardMacros.IncrementInt` (`self.TimedInputCounter`))))

(event `Key|SpaceBar` :consume false :overrideparent false
  (params (Key :type "Key Structure"))
  (:`Pressed`
    (`/Engine/EditorBlueprintResources/StandardMacros.IncrementInt` (`self.TimedInputCounter`))))

(event `SaveDataPhoto`
  (bind _value (message `/Game/Blueprints/BPI_UserData.GetAveragePawnSpeed` (`GameplayStatics.GetGameInstance`)))
  (bind _value_2 (message `/Game/Blueprints/BPI_UserData.GetAverageFastTurnCount` (`GameplayStatics.GetGameInstance`)))
  (bind _value_3 (message `/Game/Blueprints/BPI_UserData.GetAverageTurnSpeed` (`GameplayStatics.GetGameInstance`)))
  (bind _value_4 (message `/Game/Blueprints/BPI_UserData.GetAverageInputCount` (`GameplayStatics.GetGameInstance`)))
  (`self.MakeSnapshot` _value _value_2 _value_3 _value_4))

(fn `AddFastTurn`
  (bind _returnvalue (`self.GetPawnPoint`))
  (bind (_value _returnvalue_2) (`BlueprintMapLibrary.Map_Find` (`self.FastTurnData`) _returnvalue))
  (if _returnvalue_2
    (`BlueprintMapLibrary.Map_Add` (`self.FastTurnData`) _returnvalue (+ _value 1))
    (else
      (`BlueprintMapLibrary.Map_Add` (`self.FastTurnData`) _returnvalue 1))))

(fn `AddInputData`
  (bind _returnvalue (`self.GetPawnPoint`))
  (bind (_value _returnvalue_2) (`BlueprintMapLibrary.Map_Find` (`self.InputData`) _returnvalue))
  (bind _returnvalue_3 (* (`self.TimedInputCounter`) (`self.boost`)))
  (`|ExecutionSequence`
    (:`then_0`
      (if _returnvalue_2
        (if (< _value _returnvalue_3)
          (`BlueprintMapLibrary.Map_Add` (`self.InputData`) _returnvalue _returnvalue_3))
        (else
          (`BlueprintMapLibrary.Map_Add` (`self.InputData`) _returnvalue _returnvalue_3))))
    (:`then_1`
      (set `self.TimedInputCounter` 0))))

(fn `AddPawnSpeedData`
  (bind _returnvalue (`self.GetPawnPoint`))
  (bind (_value _returnvalue_2) (`BlueprintMapLibrary.Map_Find` (`self.PawnSpeedData`) _returnvalue))
  (bind _returnvalue_3 (* (`KismetMathLibrary.VSize` (`Actor.GetVelocity` (`Controller.K2_GetPawn` (`self.PlayerControllerOwner`)))) (`self.boost`)))
  (if _returnvalue_2
    (if (< _value _returnvalue_3)
      (`BlueprintMapLibrary.Map_Add` (`self.PawnSpeedData`) _returnvalue _returnvalue_3))
    (else
      (`BlueprintMapLibrary.Map_Add` (`self.PawnSpeedData`) _returnvalue _returnvalue_3))))

(fn `CalculateTurnSpeed`
  (bind _returnvalue (`self.GetPawnPoint`))
  (bind (_value _returnvalue_2) (`BlueprintMapLibrary.Map_Find` (`self.TurnSpeedData`) _returnvalue))
  (bind _returnvalue_3 (* (`KismetMathLibrary.Abs` (.yaw (`KismetMathLibrary.NormalizedDeltaRotator` (`Controller.GetControlRotation` (`self.PlayerControllerOwner`)) (`self.lastRotation`)))) (`self.boost`)))
  (if _returnvalue_2
    (if (< _value _returnvalue_3)
      (`BlueprintMapLibrary.Map_Add` (`self.TurnSpeedData`) _returnvalue _returnvalue_3))
    (else
      (`BlueprintMapLibrary.Map_Add` (`self.TurnSpeedData`) _returnvalue _returnvalue_3))))

(fn `CheckFastTurn`
  (`|ExecutionSequence`
    (:`then_0`
      (if (>= (* (`KismetMathLibrary.Abs` (.yaw (`KismetMathLibrary.NormalizedDeltaRotator` (`Controller.GetControlRotation` (`self.PlayerControllerOwner`)) (`self.lastRotation`)))) (`self.boost`)) 45.0)
        (`self.AddFastTurn`)))
    (:`then_1`
      (set `self.lastRotation` (`Controller.GetControlRotation` (`self.PlayerControllerOwner`))))))

(fn `GetPawnPoint`
  (returns (ReturnValue :type "IntPoint Structure"))
  (return (`KismetMathLibrary.Conv_Vector2DToIntPoint` (`KismetMathLibrary.Conv_VectorToVector2D` (`KismetMathLibrary.Vector_SnappedToGrid` (`Actor.K2_GetActorLocation` (`Controller.K2_GetPawn` (`GameplayStatics.GetPlayerController` 0))) (`self.PrecisionGrid`))))))

(fn `MakeSnapshot`
  (params (averagePawnSpeed :type "Float (double-precision)") (averageFastTurn :type "Float (double-precision)") (averageTurnSpeed :type "Float (double-precision)") (averageInputCount :type "Float (double-precision)"))
  (locals (PawnPoints :type "Array of IntPoint Structure") (CurrentAverageHeatValue :type "Float (double-precision)") (CurrentPoint :type "IntPoint Structure") (HeatData :type "Map of IntPoint Structure to Float (double-precision)"))
  (`|ExecutionSequence`
    (:`then_0`
      (bind _keys (`BlueprintMapLibrary.Map_Keys` (`self.PawnSpeedData`)))
      (set `local.PawnPoints` _keys)
      (bind _keys_2 (`BlueprintMapLibrary.Map_Keys` (`self.FastTurnData`)))
      (`KismetArrayLibrary.Array_Append` (`local.PawnPoints`) _keys_2)
      (bind _keys_3 (`BlueprintMapLibrary.Map_Keys` (`self.TurnSpeedData`)))
      (`KismetArrayLibrary.Array_Append` (`local.PawnPoints`) _keys_3)
      (bind _keys_4 (`BlueprintMapLibrary.Map_Keys` (`self.InputData`)))
      (`KismetArrayLibrary.Array_Append` (`local.PawnPoints`) _keys_4))
    (:`then_1`
      (for _array_element (`local.PawnPoints`)
        (set `local.CurrentPoint` _array_element)
        (`|ExecutionSequence`
          (:`then_0`
            (set `local.CurrentAverageHeatValue` (+ (`local.CurrentAverageHeatValue`) (* (`KismetMathLibrary.FClamp` (- (`BlueprintMapLibrary.Map_Find` (`self.PawnSpeedData`) (`local.CurrentPoint`)) (`local.averagePawnSpeed`))) 1.0))))
          (:`then_1`
            (set `local.CurrentAverageHeatValue` (+ (`local.CurrentAverageHeatValue`) (* (`KismetMathLibrary.FClamp` (- (`KismetMathLibrary.Conv_IntToDouble` (`BlueprintMapLibrary.Map_Find` (`self.FastTurnData`) (`local.CurrentPoint`))) (`local.averageFastTurn`))) 1.0))))
          (:`then_2`
            (set `local.CurrentAverageHeatValue` (+ (`local.CurrentAverageHeatValue`) (* (`KismetMathLibrary.FClamp` (- (`BlueprintMapLibrary.Map_Find` (`self.TurnSpeedData`) (`local.CurrentPoint`)) (`local.averageTurnSpeed`))) 1.0))))
          (:`then_3`
            (set `local.CurrentAverageHeatValue` (+ (`local.CurrentAverageHeatValue`) (* (`KismetMathLibrary.FClamp` (- (`BlueprintMapLibrary.Map_Find` (`self.InputData`) (`local.CurrentPoint`)) (`local.averageInputCount`))) 1.0))))
          (:`then_4`
            (set `local.CurrentAverageHeatValue` (/ (`local.CurrentAverageHeatValue`) 4.0)))
          (:`then_5`
            (`BlueprintMapLibrary.Map_Add` (`local.HeatData`) (`local.CurrentPoint`) (`local.CurrentAverageHeatValue`))))))
    (:`then_2`
      (bind _keys_5 (`BlueprintMapLibrary.Map_Keys` (`local.HeatData`)))
      (for _array_element_2 _keys_5
        (`|SpawnActorFromClass` "/Game/Blueprints/Statistics/BP_ProbeActor.BP_ProbeActor_C" (`KismetMathLibrary.MakeTransform` (`KismetMathLibrary.Conv_Vector2DToVector` (`KismetMathLibrary.Conv_IntPointToVector2D` _array_element_2))) "AlwaysSpawn" "MultiplyWithRoot" null (`BlueprintMapLibrary.Map_Find` (`local.HeatData`) _array_element_2) null)))
    (:`then_3`
      (bind _outactors (`GameplayStatics.GetAllActorsWithTag` "Snapshot"))
      (`|SpawnActorFromClass` "/Game/Blueprints/Statistics/BP_SnapshotCamera.BP_SnapshotCamera_C" (`Actor.GetTransform` (`|GetArrayItem` _outactors)) "AlwaysSpawn" "MultiplyWithRoot" null null))))