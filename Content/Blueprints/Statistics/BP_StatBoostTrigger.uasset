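; BP_StatBoostTrigger is a trigger volume that changes the Boost value on a user statistics component while an actor is inside its box.
; Begin overlap finds BP_UserStatisticsComponent on the overlapping actor's instigator controller and applies the trigger's Boost.
; The first valid entry also plays ScreamerSound once at the trigger's location.
; End overlap resets the component's Boost to a neutral 1.0 rather than restoring its previous value.
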(event `self.Box.OnComponentBeginOverlap`
  (params (OverlappedComponent :type "PrimitiveComponent Object Reference") (OtherActor :type "Actor Object Reference") (OtherComp :type "PrimitiveComponent Object Reference") (OtherBodyIndex :type Integer) (bFromSweep :type Boolean) (SweepResult :type "HitResult Structure (by ref)"))
  (bind _returnvalue (`self.GetComponentByClass` (`self.GetInstigatorController` OtherActor) "/Game/Blueprints/Statistics/BP_UserStatisticsComponent.BP_UserStatisticsComponent_C"))
  (`/Engine/EditorBlueprintResources/StandardMacros.IsValid` _returnvalue
    (:`Is Valid`
      (set `/Game/Blueprints/Statistics/BP_UserStatisticsComponent.boost` (`self.Boost`) _returnvalue)
      (`/Engine/EditorBlueprintResources/StandardMacros.DoOnce` false
        (:`Completed`
          (`GameplayStatics.PlaySoundAtLocation` (`self.ScreamerSound`) (`self.K2_GetActorLocation`) (struct) 1.0 1.0 0.0 null null null null))))))

(event `self.Box.OnComponentEndOverlap`
  (params (OverlappedComponent :type "PrimitiveComponent Object Reference") (OtherActor :type "Actor Object Reference") (OtherComp :type "PrimitiveComponent Object Reference") (OtherBodyIndex :type Integer))
  (bind _returnvalue (`self.GetComponentByClass` (`self.GetInstigatorController` OtherActor) "/Game/Blueprints/Statistics/BP_UserStatisticsComponent.BP_UserStatisticsComponent_C"))
  (`/Engine/EditorBlueprintResources/StandardMacros.IsValid` _returnvalue
    (:`Is Valid`
      (set `/Game/Blueprints/Statistics/BP_UserStatisticsComponent.boost` 1.0 _returnvalue))))

(fn `UserConstructionScript`)