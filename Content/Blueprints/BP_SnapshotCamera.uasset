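; One-shot snapshot camera actor that saves a scene capture as a timestamped PNG in the project directory.
; On BeginPlay it creates a square render target for its SceneCaptureComponent2D, then chains two short timers to enable capture and export the image.
; After export it disables capture, destroys every BP_ProbeActor in the level and then destroys itself.
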(event `self.ReceiveBeginPlay`
  (bind _returnvalue (`KismetRenderingLibrary.CreateRenderTarget2D` 1080 1080 "RTF_RGBA8"))
  (set `self.Texture Target` _returnvalue)
  (set `SceneCaptureComponent2D.TextureTarget` (`self.Texture Target`) (`self.SceneCaptureComponent2D`))
  (`KismetSystemLibrary.K2_SetTimerDelegate` (delegate `PreparePhoto`) 0.01))

(event `PreparePhoto`
  (set `SceneCaptureComponent.bCaptureEveryFrame` true (`self.SceneCaptureComponent2D`))
  (`KismetSystemLibrary.K2_SetTimerDelegate` (delegate `TakePhoto`) 0.01))

(event `TakePhoto`
  (bind (_seconds _partialseconds) (`GameplayStatics.GetAccurateRealTime`))
  (`KismetRenderingLibrary.ExportRenderTarget` (`self.Texture Target`) (`KismetSystemLibrary.GetProjectDirectory`) (`KismetStringLibrary.Concat_StrStr` (`KismetStringLibrary.Conv_IntToString` _seconds) (`KismetStringLibrary.Conv_DoubleToString` _partialseconds) ".png"))
  (set `SceneCaptureComponent.bCaptureEveryFrame` false (`self.SceneCaptureComponent2D`))
  (bind _outactors (`GameplayStatics.GetAllActorsOfClass` "/Game/Blueprints/BP_ProbeActor.BP_ProbeActor_C"))
  (for _array_element _outactors
    (`self.K2_DestroyActor` _array_element))
  (`self.K2_DestroyActor`))

(fn `UserConstructionScript`)