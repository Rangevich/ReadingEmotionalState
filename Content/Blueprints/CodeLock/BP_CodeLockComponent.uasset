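; Code lock component that generates a random zero-padded four-digit code and fires an opened event when its numpads match it.
; On BeginPlay it maps provider actors by numpad position and binds their selection events, each triggering a digit-by-digit check.
; It spawns a hint per digit at randomly picked "SpawnCode"-tagged actors, colored like the matching numpad to convey order, then destroys the unpicked spawn actors.
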(event `self.ReceiveBeginPlay`
  (`self.RandomCode`)
  (for _array_element (`self.CodeProviders`)
    (bind _returnvalue (`Actor.GetComponentByClass` _array_element "/Game/Blueprints/CodeLock/BP_NumpadComponent.BP_NumpadComponent_C"))
    (add `/Game/Blueprints/CodeLock/BP_NumpadComponent.OnSelected` _returnvalue (delegate `SelectedEvent`))
    (`BlueprintMapLibrary.Map_Add` (`self.providerSort`) (`/Game/Blueprints/CodeLock/BP_NumpadComponent.position` _returnvalue) _array_element))
  (`self.SpawnHints`))

(event `SelectedEvent`
  (`self.ApplyCode`))

(event `ApplyCode`
  (for (_array_element _array_index) (`KismetStringLibrary.GetCharacterArrayFromString` (`self.Code`))
    (bind _returnvalue (`Actor.GetComponentByClass` (`BlueprintMapLibrary.Map_Find` (`self.providerSort`) _array_index) "/Game/Blueprints/CodeLock/BP_NumpadComponent.BP_NumpadComponent_C"))
    (if (and (== _array_index (`/Game/Blueprints/CodeLock/BP_NumpadComponent.position` _returnvalue)) (`KismetStringLibrary.EqualEqual_StrStr` _array_element (`/Game/Blueprints/CodeLock/BP_NumpadComponent.selectedCharacter` _returnvalue)))
      (`/Engine/EditorBlueprintResources/StandardMacros.IncrementInt` (`self.check`))))
  (`|ExecutionSequence`
    (:`then_0`
      (if (== (`self.check`) (`KismetArrayLibrary.Array_Length` (`KismetStringLibrary.GetCharacterArrayFromString` (`self.Code`))))
        (`self.OnCodeLockOpened`)))
    (:`then_1`
      (set `self.check` 0))))

(fn `RandomCode`
  (locals (localCode :type String) (number :type Integer :default 0))
  (bind _output_get (set `local.number` (`KismetMathLibrary.RandomIntegerInRange` 0 9999)))
  (bind _output_get_2 (set `local.localCode` (`KismetStringLibrary.Conv_IntToString` _output_get)))
  (while (< (`KismetStringLibrary.Len` _output_get_2) 4)
    (set `local.localCode` (`KismetStringLibrary.Concat_StrStr` "0" (`local.localCode`))))
  (set `self.Code` (`local.localCode`)))

(fn `SpawnHints`
  (locals (potentialSpawnPlaces :type "Array of Actor Object Reference") (selectedSpawnPlaces :type "Array of Actor Object Reference") (selectedPlace :type "Actor Object Reference") (codeData :type "Array of String"))
  (`|ExecutionSequence`
    (:`then_0`
      (bind _outactors (`GameplayStatics.GetAllActorsWithTag` "SpawnCode"))
      (set `local.potentialSpawnPlaces` _outactors)
      (for _ (range 4)
        (bind _output_get (set `local.selectedPlace` (`KismetArrayLibrary.Array_Random` (`local.potentialSpawnPlaces`))))
        (`KismetArrayLibrary.Array_Add` (`local.selectedSpawnPlaces`) _output_get)
        (`KismetArrayLibrary.Array_RemoveItem` (`local.potentialSpawnPlaces`) (`local.selectedPlace`)))
      (set `local.codeData` (`KismetStringLibrary.GetCharacterArrayFromString` (`self.Code`)))
      (for (_array_element _array_index) (`local.selectedSpawnPlaces`)
        (`|SpawnActorFromClass` "/Game/Blueprints/CodeLock/BP_CodeHint.BP_CodeHint_C" (`Actor.GetTransform` _array_element) "AlwaysSpawn" "MultiplyWithRoot" null (`KismetTextLibrary.Conv_StringToText` (`|GetArrayItem` (`local.codeData`) _array_index)) (`KismetMathLibrary.Conv_LinearColorToColor` (`/Game/Blueprints/CodeLock/BP_NumpadComponent.Color` (`Actor.GetComponentByClass` (`BlueprintMapLibrary.Map_Find` (`self.providerSort`) _array_index) "/Game/Blueprints/CodeLock/BP_NumpadComponent.BP_NumpadComponent_C"))) null)))
    (:`then_1`
      (for _array_element_2 (`local.potentialSpawnPlaces`)
        (`Actor.K2_DestroyActor` _array_element_2)))))